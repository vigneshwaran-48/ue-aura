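; BP_WeaponEquipment_Base is a weapon equipment base that swaps the owning character's animation overlay.
; On equip, it fetches the owner's primary skeletal mesh through a message call, caches it and links the WeaponOverlay anim class layers.
; An invalid mesh prints an error string instead.
; On unequip, it relinks the cached mesh to the default overlay pose, ABP_OverlayPose_Default.
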(event EventOnEquipped
  (params (ASC :type Aura%20Ability%20System%20Component%20Object%20Reference))
  (bind _skeletalmesh (Class|BPICharacter|GetPrimarySkeletalMesh(Message) (Variables|Default|GetOwningActor)))
  (Utilities|IsValid _skeletalmesh
    (:Is%20Valid
      (bind _output_get (Variables|Default|SetPrimarySkeletalMesh _skeletalmesh))
      (Components|SkeletalMesh|AnimationBlueprintLinking|LinkAnimClassLayers _output_get (Variables|Overlay|GetWeaponOverlay)))
    (:Is%20Not%20Valid
      (Development|PrintString 0 "Primary Skeletal Mesh is Invalid"))))

(event EventOnUnequipped
  (params (ASC :type Aura%20Ability%20System%20Component%20Object%20Reference))
  (bind _primaryskeletalmesh (Variables|Default|GetPrimarySkeletalMesh))
  (Utilities|IsValid _primaryskeletalmesh
    (:Is%20Valid
      (Components|SkeletalMesh|AnimationBlueprintLinking|LinkAnimClassLayers _primaryskeletalmesh "/AuraFramework/Animation/OverlaySystem/Overlays/Poses/Default/ABP_OverlayPose_Default.ABP_OverlayPose_Default_C"))))